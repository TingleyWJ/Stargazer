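; Squadron is an AI starship Blueprint that carries an overlay widget on a WidgetComponent.
; On BeginPlay it casts that widget to AIOverlay and sets itself as the overlay's OwnerStarship.
; Tick is empty, and a disconnected node chain that would rotate the widget toward the player camera never runs.
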(event EventBeginPlay
  (bind _asaioverlay (Utilities|Casting|CastToAIOverlay (UserInterface|GetUserWidgetObject (Variables|Default|GetWidgetComponent))))
  (Variables|/Game/Blueprints/UI/AIOverlay.AIOverlay_C|SetOwnerStarship _asaioverlay self))

(event EventTick
  (params (DeltaSeconds :type Float%20%28single-precision%29)))

(fn ConstructionScript)