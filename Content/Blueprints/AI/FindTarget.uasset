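; FindTarget is a behavior tree node that picks a target for AI starships.
; Each tick it uses the AIStarshipController, cached on first run, to sphere-trace for Pawns in a large radius around the controlled pawn.
; The hit actor is written to the Target blackboard key, which is cleared on a miss.
; AIStarshipBase actors are ignored, except on the caching tick, which skips gathering that list.
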(event EventTick
  (params (OwnerActor :type Actor%20Object%20Reference) (DeltaSeconds :type Float%20%28single-precision%29))
  (bind _target (Variables|Default|GetTarget))
  (Utilities|IsValid (Variables|Default|GetAIController)
    (:Is%20Valid
      (bind _outactors (Actor|GetAllActorsOfClass "/Script/Stargazer.AIStarshipBase")))
    (:Is%20Not%20Valid
      (bind _asaistarship_controller (Utilities|Casting|CastToAIStarshipController OwnerActor))
      (Variables|Default|SetAIController _asaistarship_controller)))
  (bind (_outhit _returnvalue) (Collision|SphereTraceForObjects (Transformation|GetActorLocation (Pawn|GetControlledPawn (Variables|Default|GetAIController))) (Transformation|GetActorLocation (Pawn|GetControlledPawn (Variables|Default|GetAIController))) 7.5e+03 (Utilities|Array|MakeArray "ObjectTypeQuery3") false _outactors "None"))
  (if _returnvalue
    (Class|BTFunctionLibrary|SetBlackboardValueasObject _target (.HitActor (Collision|BreakHitResult _outhit)))
    (else
      (Class|BTFunctionLibrary|SetBlackboardValueasObject _target))))